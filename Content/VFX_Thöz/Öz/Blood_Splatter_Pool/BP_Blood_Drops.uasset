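; Blood drop effect actor that leaves blood decals in the world from particle data exported by its Niagara blood effect.
; On BeginPlay it passes itself to the Niagara system as the callback object for particle data.
; Each received particle spawns a decal at its position, oriented against its velocity and randomly scaled up to the set decal size.
; Each decal fades out after a short delay.
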(event Collision|EventActorBeginOverlap
  (params (OtherActor :type Actor%20Object%20Reference)))

(event EventParticleData
  (params (Data :type Array%20of%20Basic%20Particle%20Data%20Structures) (NiagaraSystem :type Niagara%20System%20Object%20Reference) (SimulationPositionOffset :type Vector%20%28by%20ref%29 :default "0, 0, 0"))
  (bind _decalsize (Variables|Default|GetDecalSize))
  (for _array_element Data
    (bind _returnvalue (Rendering|Decal|SpawnDecalatLocation "/Game/VFX_Thöz/Öz/Blood_Splatter_Pool/Decal_blood_M_Inst.Decal_blood_M_Inst" (Math|Conversions|ToVector(Float) (Math|Float|Lerp (* _decalsize 0.1) _decalsize (Math|Random|RandomFloatinRange 0.0 1.0))) (.Position (Utilities|Struct|BreakBasicParticleData _array_element)) (Math|Conversions|RotationFromXVector (* (.Velocity (Utilities|Struct|BreakBasicParticleData _array_element)) -1.0)) 0.0))
    (Rendering|Components|Decal|SetFadeOut _returnvalue 3.0 5.0 true)))

(event EventTick
  (params (DeltaSeconds :type Float%20%28single-precision%29)))

(event EventBeginPlay
  (Class|NiagaraComponent|SetVariableObject (Variables|Default|GetNS_Blood_Effect) "BP_Blood" self))

(fn ConstructionScript)