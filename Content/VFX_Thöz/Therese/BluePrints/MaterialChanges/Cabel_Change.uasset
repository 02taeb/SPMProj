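; Interactive cable material-change actor that lets the player press M inside a trigger box to switch its static mesh to the El material.
; Box overlap enables or disables player input and toggles a text render's visibility.
; A delayed Tick acts as a seconds counter, reset on each press, that applies the black cloud material once it passes five.
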(event OnComponentBeginOverlap(Box)
  (params (OverlappedComponent :type Primitive%20Component%20Object%20Reference) (OtherActor :type Actor%20Object%20Reference) (OtherComp :type Primitive%20Component%20Object%20Reference) (OtherBodyIndex :type Integer) (bFromSweep :type Boolean) (SweepResult :type Hit%20Result%20Structure%20%28by%20ref%29))
  (Input|EnableInput (Game|GetPlayerController 0))
  (Rendering|ToggleVisibility (Variables|Default|GetTextRender) false))

(event OnComponentEndOverlap(Box)
  (params (OverlappedComponent :type Primitive%20Component%20Object%20Reference) (OtherActor :type Actor%20Object%20Reference) (OtherComp :type Primitive%20Component%20Object%20Reference) (OtherBodyIndex :type Integer))
  (Input|DisableInput (Game|GetPlayerController 0))
  (Rendering|ToggleVisibility (Variables|Default|GetTextRender) false))

(event EventBeginPlay)

(event Collision|EventActorBeginOverlap
  (params (OtherActor :type Actor%20Object%20Reference)))

(event EventTick
  (params (DeltaSeconds :type Float%20%28single-precision%29))
  (Utilities|FlowControl|Delay 1.0)
  (Variables|Components|SetSeconds (+ (Variables|Components|GetSeconds) 1))
  (if (and (Variables|Default|GetKlickedButton) (> (Variables|Components|GetSeconds) 5))
    (Rendering|Material|SetMaterial (Variables|Default|GetStaticMesh) 0 "/Game/VFX_Thöz/Therese/Shaders/Cloud/Cloud_M_black_Inst.Cloud_M_black_Inst")))

(event Input|KeyboardEvents|M
  (params (Key :type Key%20Structure))
  (:Pressed
    (Rendering|Material|SetMaterial (Variables|Default|GetStaticMesh) 0 "/Game/VFX_Thöz/Therese/Shaders/El/El.El")
    (Variables|Default|SetKlickedButton true)
    (Variables|Components|SetSeconds 0)))

(fn ConstructionScript)