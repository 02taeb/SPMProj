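; Blood effect actor that turns Niagara particle data into fading blood decals in the world.
; On BeginPlay it registers itself with its Niagara component through the "BP Blood" object variable, so the system can export particle data back to it.
; Each exported particle spawns a decal at its position, oriented against its velocity, which fades out after a short delay.
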(event EventBeginPlay
  (Class|NiagaraComponent|SetVariableObject (Variables|Default|GetNiagara) "BP Blood" self))

(event Collision|EventActorBeginOverlap
  (params (OtherActor :type Actor%20Object%20Reference)))

(event EventTick
  (params (DeltaSeconds :type Float%20%28single-precision%29)))

(event EventParticleData
  (params (Data :type Array%20of%20Basic%20Particle%20Data%20Structures) (NiagaraSystem :type Niagara%20System%20Object%20Reference) (SimulationPositionOffset :type Vector%20%28by%20ref%29 :default "0, 0, 0"))
  (for _array_element Data
    (bind _returnvalue (Rendering|Decal|SpawnDecalatLocation "/Game/VFX_Thöz/Therese/Decals/Blood/Blod_decal_fade.Blod_decal_fade" (Math|Conversions|ToVector(Float) (Variables|Default|GetDecalsSize)) (.Position (Utilities|Struct|BreakBasicParticleData _array_element)) (Math|Conversions|RotationFromXVector (* (.Velocity (Utilities|Struct|BreakBasicParticleData _array_element)) -1.0)) 1e+01))
    (Rendering|Components|Decal|SetFadeOut _returnvalue 3.0 5.0 true)))

(fn ConstructionScript)