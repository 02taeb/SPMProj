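; An interactable elevator component that teleports whoever interacts with it to a TeleportTo location behind a screen fade.
; On Interact it plays a crystal sound at the owner, disables the instigator's input and fades the camera out.
; After a fixed one-second delay, independent of FadeTime, it moves the instigator without sweeping, starts the fade back in and immediately re-enables input.
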(event EventInteract
  (params (Instigator :type Actor%20Object%20Reference))
  (bind _returnvalue (Game|GetPlayerCameraManager 0))
  (Audio|PlaySoundatLocation "/Game/Audio/Crystal_Attack.Crystal_Attack" (Transformation|GetActorLocation (Components|GetOwner)) "0, 0, 0" 1.0 1.0 0.0 0 0 0 0)
  (Input|DisableInput Instigator 0)
  (CameraFades|StartCameraFade :self _returnvalue :ToAlpha 1.0 :Duration (Variables|Default|GetFadeTime) :bHoldWhenFinished true)
  (Utilities|FlowControl|Delay 1.0)
  (Transformation|SetActorLocation Instigator (Variables|Default|GetTeleportTo) false true)
  (CameraFades|StartCameraFade :self _returnvalue :FromAlpha 1.0 :Duration (Variables|Default|GetFadeTime))
  (Input|EnableInput Instigator 0))