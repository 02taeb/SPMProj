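; Interactable loot component for parasite chests that grants the player one random HP, Def or Atk parasite when interacted with.
; Interact checks the player's InventoryComponent; if full, it briefly shows an inventory-full widget.
; Otherwise it spawns a random parasite, opens the owning BP_ParChest, marks itself looted and casts the parasite to call AddToInventory.
; Both notification widgets clear existing copies before showing for three seconds.
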(event EventInteract
  (params (Instigator :type Actor%20Object%20Reference))
  (if (not (Variables|Default|GetLooted))
    (bind _asbp_player_character (Utilities|Casting|CastToBP_PlayerCharacter Instigator))
    (bind _returnvalue (Class|InventoryComponent|IsFull (Actor|GetComponentbyClass _asbp_player_character "/Script/SPMProj.InventoryComponent")))
    (if _returnvalue
      (bind _foundwidgets (Widget|GetAllWidgetsOfClass "/Game/Blueprints/UI/WBP_InventoryFull.WBP_InventoryFull_C" true))
      (for _array_element _foundwidgets
        (Widget|RemovefromParent _array_element))
      (bind _returnvalue_2 (UserInterface|CreateWidget "/Game/Blueprints/UI/WBP_InventoryFull.WBP_InventoryFull_C" (Game|GetPlayerController 0)))
      (UserInterface|Viewport|AddtoViewport _returnvalue_2 0)
      (Utilities|FlowControl|Delay 3.0)
      (Widget|RemovefromParent _returnvalue_2)
      (elif (not (Variables|Default|GetLooted))
        (bind _returnvalue_3 (Game|SpawnActorfromClass (.OutItem (Utilities|Array|Random (Utilities|Array|MakeArray (Variables|Default|GetHPParasite) (Variables|Default|GetDefParasite) (Variables|Default|GetAtkParasite)))) (Math|Transform|MakeTransform "0, 0, 0" "0, 0, 0" "1.000000,1.000000,1.000000") "Undefined" 0 0))
        (Utilities|FlowControl|Sequence
          (:then_0
            (bind _asbp_par_chest (Utilities|Casting|CastToBP_ParChest (Components|GetOwner)))
            (Default|Open _asbp_par_chest)
            (Variables|Default|SetLooted true))
          (:then_1
            (bind _asbp_def_parasite (Utilities|Casting|CastToBP_DefParasite _returnvalue_3)
              (:then
                (Default|AddtoInventory _asbp_def_parasite))
              (:CastFailed
                (bind _asbp_atk_parasite (Utilities|Casting|CastToBP_AtkParasite _returnvalue_3)
                  (:then
                    (Default|AddtoInventory _asbp_atk_parasite))
                  (:CastFailed
                    (bind _asbp_hpparasite (Utilities|Casting|CastToBP_HPParasite _returnvalue_3))
                    (Default|AddtoInventory _asbp_hpparasite))))))
          (:then_2
            (bind _foundwidgets_2 (Widget|GetAllWidgetsOfClass "/Game/Blueprints/UI/WBP_AddedToInv.WBP_AddedToInv_C" true))
            (for _array_element_2 _foundwidgets_2
              (Widget|RemovefromParent _array_element_2))
            (bind _returnvalue_4 (UserInterface|CreateWidget "/Game/Blueprints/UI/WBP_AddedToInv.WBP_AddedToInv_C" (Game|GetPlayerController 0)))
            (UserInterface|Viewport|AddtoViewport _returnvalue_4 0)
            (Utilities|FlowControl|Delay 3.0)
            (Widget|RemovefromParent _returnvalue_4)))))))