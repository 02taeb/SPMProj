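; BP_ParChest is an interactable chest that the player can open once.
; Overlapping its Box creates an interact prompt widget for the player while the chest is unlooted, and leaving removes it.
; The Open event, which nothing in this graph calls, rolls the Cube mesh by a fixed angle, sets Looted and plays a 2D sound.
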(event OnComponentBeginOverlap(Box)
  (params (OverlappedComponent :type Primitive%20Component%20Object%20Reference) (OtherActor :type Actor%20Object%20Reference) (OtherComp :type Primitive%20Component%20Object%20Reference) (OtherBodyIndex :type Integer) (bFromSweep :type Boolean) (SweepResult :type Hit%20Result%20Structure%20%28by%20ref%29))
  (if (not (Variables|Default|GetLooted))
    (bind _asbp_player_character (Utilities|Casting|CastToBP_PlayerCharacter OtherActor))
    (bind _asplayer_controller (Utilities|Casting|CastToPlayerController (Pawn|GetController _asbp_player_character)))
    (bind _returnvalue (UserInterface|CreateWidget "/Game/Blueprints/UI/WBP_InteractPrompt.WBP_InteractPrompt_C" _asplayer_controller))
    (UserInterface|Viewport|AddtoViewport _returnvalue 0)
    (Variables|Default|SetWidget true)))

(event OnComponentEndOverlap(Box)
  (params (OverlappedComponent :type Primitive%20Component%20Object%20Reference) (OtherActor :type Actor%20Object%20Reference) (OtherComp :type Primitive%20Component%20Object%20Reference) (OtherBodyIndex :type Integer))
  (if (Variables|Default|GetWidget)
    (Utilities|Casting|CastToBP_PlayerCharacter OtherActor)
    (Widget|RemovefromParent (stale OnComponentBeginOverlap(Box) _returnvalue))
    (Variables|Default|SetWidget false)))

(event Custom|Open
  (bind _cube (Variables|Default|GetCube))
  (bind _returnvalue (Transformation|GetWorldRotation _cube))
  (if (not (Variables|Default|GetLooted))
    (Transformation|SetWorldRotation _cube (Math|Rotator|MakeRotator (+ (.roll _returnvalue) -3e+01) (.pitch _returnvalue) (.yaw _returnvalue)) false false)
    (Variables|Default|SetLooted true)
    (Audio|PlaySound2D "/Game/Sound/ParasiteDialogue/MoreOfMyBrothersJoinUs.MoreOfMyBrothersJoinUs" 5.0 1.0 0.0 0 0)))

(fn ConstructionScript)