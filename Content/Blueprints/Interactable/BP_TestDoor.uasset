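; BP_TestDoor is an interactable door that swings open and closed around its yaw axis with sound.
; Activate and Deactivate set the IsActivated flag and play the matching open or close sound at the actor's location with attenuation.
; Tick polls that flag every frame to play or reverse a timeline, whose update scales the door mesh's relative yaw.
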(event EventTick
  (params (DeltaSeconds :type Float%20%28single-precision%29))
  (if (Variables|Default|GetisActivated)
    (bind _door (Timeline|Timeline Play)
      (:Update
        (Transformation|SetRelativeRotation (Variables|Default|GetDoor) (Math|Rotator|MakeRotator 0.0 0.0 (* _door -104.0)) false false)))
    (else
      (Timeline|Timeline Reverse))))

(fn ConstructionScript)

(fn Activate
  (Variables|Default|SetisActivated true)
  (Audio|PlaySoundatLocation "/Game/Audio/Interact/DoorOpen.DoorOpen" (Transformation|GetActorLocation) "0, 0, 0" 1.0 1.0 0.0 "/Game/Audio/Interact/SoundAttenuation.SoundAttenuation" 0 0 0))

(fn Deactivate
  (Variables|Default|SetisActivated false)
  (Audio|PlaySoundatLocation "/Game/Audio/Interact/DoorClose.DoorClose" (Transformation|GetActorLocation) "0, 0, 0" 1.0 1.0 0.0 "/Game/Audio/Interact/SoundAttenuation.SoundAttenuation" 0 0 0))