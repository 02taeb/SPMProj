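; Interactable book pile actor that shows an interact prompt while the player character is inside its box trigger.
; Overlap begin creates a WBP_InteractPrompt widget for that character's player controller and adds it to the viewport.
; Overlap end removes the prompt and also closes any valid note widget held by BPInteractableNoteComponent, resetting its IsOpen flag.
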(event OnComponentEndOverlap(Box)
  (params (OverlappedComponent :type Primitive%20Component%20Object%20Reference) (OtherActor :type Actor%20Object%20Reference) (OtherComp :type Primitive%20Component%20Object%20Reference) (OtherBodyIndex :type Integer))
  (bind _bp_interactablenotecomponent (Variables|Default|GetBP_InteractableNoteComponent))
  (bind _widget (Variables|/Game/Blueprints/Interactable/BP_InteractableNoteComponent.BP_InteractableNoteComponent_C|GetWidget _bp_interactablenotecomponent))
  (Utilities|Casting|CastToPlayerCharacter OtherActor)
  (Utilities|IsValid _widget
    (:Is%20Valid
      (Widget|RemovefromParent _widget)
      (Variables|/Game/Blueprints/Interactable/BP_InteractableNoteComponent.BP_InteractableNoteComponent_C|SetIsOpen _bp_interactablenotecomponent false))
    (:Is%20Not%20Valid
      _))
  (Widget|RemovefromParent (stale OnComponentBeginOverlap(Box) _returnvalue)))

(event OnComponentBeginOverlap(Box)
  (params (OverlappedComponent :type Primitive%20Component%20Object%20Reference) (OtherActor :type Actor%20Object%20Reference) (OtherComp :type Primitive%20Component%20Object%20Reference) (OtherBodyIndex :type Integer) (bFromSweep :type Boolean) (SweepResult :type Hit%20Result%20Structure%20%28by%20ref%29))
  (bind _asplayer_character (Utilities|Casting|CastToPlayerCharacter OtherActor))
  (bind _asplayer_controller (Utilities|Casting|CastToPlayerController (Pawn|GetController _asplayer_character)))
  (bind _returnvalue (UserInterface|CreateWidget "/Game/Blueprints/UI/WBP_InteractPrompt.WBP_InteractPrompt_C" _asplayer_controller))
  (UserInterface|Viewport|AddtoViewport _returnvalue 0))

(fn ConstructionScript)