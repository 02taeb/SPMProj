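; Actor component that makes its owning actor act as an interactable swing door, rotating it in yaw between its starting angle and a target angle.
; Interact enables rotation for RotateTime seconds, during which Tick eases the owner's yaw with RInterpTo, reusing RotateTime as interpolation speed.
; Afterwards, it targets the start yaw if the door is within one degree of its target, otherwise the original target.
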(event EventTick
  (params (DeltaSeconds :type Float%20%28single-precision%29))
  (if (Variables|Default|GetShouldRotate)
    (Transformation|SetActorRotation (Components|GetOwner) (CallFunction|ReturnRInterpOwner DeltaSeconds))))

(event EventBeginPlay
  (CallFunction|SetStartVars))

(event EventInteract
  (params (Instigator :type Actor%20Object%20Reference))
  (Variables|Default|SetShouldRotate true)
  (Utilities|FlowControl|Delay (Variables|Default|GetRotateTime))
  (Variables|Default|SetShouldRotate false)
  (CallFunction|SetNewTargetRotation))

(fn ReturnRInterpOwner
  (params (DeltaTime :type Float%20%28single-precision%29))
  (bind _returnvalue (Components|GetOwner))
  (bind _returnvalue_2 (Transformation|GetActorRotation _returnvalue))
  (return (Math|Interpolation|RInterpTo (Math|Rotator|MakeRotator (.roll _returnvalue_2) (.pitch _returnvalue_2) (.yaw _returnvalue_2)) (Math|Rotator|MakeRotator (.roll _returnvalue_2) (.pitch _returnvalue_2) (Variables|Default|GetTargetRotationZ)) DeltaTime (Variables|Default|GetRotateTime))))

(fn SetStartVars
  (Variables|Default|SetStartRotationZ (.yaw (Transformation|GetActorRotation (Components|GetOwner))))
  (Variables|Default|SetPermTargetRotationZ (Variables|Default|GetTargetRotationZ)))

(fn SetNewTargetRotation
  (if (Math|Float|NearlyEqual(Float) (.yaw (Transformation|GetActorRotation (Components|GetOwner))) (Variables|Default|GetTargetRotationZ) 1.0)
    (Variables|Default|SetTargetRotationZ (Variables|Default|GetStartRotationZ))
    (else
      (Variables|Default|SetTargetRotationZ (Variables|Default|GetPermTargetRotationZ)))))