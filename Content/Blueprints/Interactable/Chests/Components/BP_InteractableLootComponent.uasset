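; Interactable loot component for chests whose Interact event is currently empty, so it does nothing in game.
; Disconnected logic checks the player's inventory, shows a temporary full-inventory notice or spawns a random HP, Stm or Atk parasite.
; That unused path also opens the owning BP_ParChest, marks it looted, adds the parasite to inventory and shows a timed confirmation widget.
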(event EventInteract
  (params (Instigator :type Actor%20Object%20Reference)))