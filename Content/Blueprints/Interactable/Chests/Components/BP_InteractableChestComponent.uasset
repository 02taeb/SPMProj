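; Interactable component for parasite chests that gives the player a one-time parasite reward.
; On a player's Interact, it opens the owning BP_ParasiteChest and marks itself looted.
; It calls OnEat on the player's HP, ATK or DEF parasite matching ParasiteToSpawn, then briefly shows a pickup widget.
; Older spawn-to-inventory and inventory-full logic remains disconnected.
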(event EventInteract
  (params (Instigator :type Actor%20Object%20Reference))
  (if (not (Variables|Default|GetLooted))
    (Utilities|Casting|CastToBP_PlayerCharacter Instigator)
    (Utilities|FlowControl|Sequence
      (:then_0
        (bind _asbp_parasite_chest (Utilities|Casting|CastToBP_ParasiteChest (Components|GetOwner)))
        (Default|Open _asbp_parasite_chest)
        (Variables|Default|SetLooted true))
      (:then_1
        (if (== (Variables|Default|GetParasiteToSpawn) "/Game/Blueprints/Items/Parasites/BP_HPParasite.BP_HPParasite_C")
          (bind _asbp_player_character (Utilities|Casting|CastToBP_PlayerCharacter (Game|GetPlayerCharacter 0)))
          (bind _asequipable_parasite (Utilities|Casting|CastToEquipableParasite (Variables|/Script/SPMProj.PlayerCharacter|GetHPPar _asbp_player_character)))
          (Class|EquipableParasite|OnEat _asequipable_parasite)
          (elif (== (Variables|Default|GetParasiteToSpawn) "/Game/Blueprints/Items/Parasites/BP_AtkParasite.BP_AtkParasite_C")
            (bind _asbp_player_character_2 (Utilities|Casting|CastToBP_PlayerCharacter (Game|GetPlayerCharacter 0)))
            (bind _asequipable_parasite_2 (Utilities|Casting|CastToEquipableParasite (Variables|/Script/SPMProj.PlayerCharacter|GetATKPar _asbp_player_character_2)))
            (Class|EquipableParasite|OnEat _asequipable_parasite_2)
            (elif (== (Variables|Default|GetParasiteToSpawn) "/Game/Blueprints/Items/Parasites/BP_DefParasite.BP_DefParasite_C")
              (bind _asbp_player_character_3 (Utilities|Casting|CastToBP_PlayerCharacter (Game|GetPlayerCharacter 0)))
              (bind _asequipable_parasite_3 (Utilities|Casting|CastToEquipableParasite (Variables|/Script/SPMProj.PlayerCharacter|GetDEFPar _asbp_player_character_3)))
              (Class|EquipableParasite|OnEat _asequipable_parasite_3)))))
      (:then_2
        (bind _foundwidgets (Widget|GetAllWidgetsOfClass "/Game/Blueprints/UI/WBP_AddedToInv.WBP_AddedToInv_C" true))
        (for _array_element _foundwidgets
          (Widget|RemovefromParent _array_element))
        (bind _returnvalue (UserInterface|CreateWidget "/Game/Narrative/MechanicIntroductions/PickUp/PickUp.PickUp_C" (Game|GetPlayerController 0)))
        (UserInterface|Viewport|AddtoViewport _returnvalue 0)
        (Utilities|FlowControl|Delay 3.0)
        (Widget|RemovefromParent _returnvalue)))))