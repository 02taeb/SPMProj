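; Interactable note component that toggles a readable note image on screen when interacted with.
; On Interact it creates a StartingHallLetter widget for the first player controller, applies the NoteImage texture to its image and adds it to the viewport.
; A second Interact removes that widget, with an IsOpen flag tracking the state.
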(event EventInteract
  (params (Instigator :type Actor%20Object%20Reference))
  (if (Variables|Default|GetIsOpen)
    (Widget|RemovefromParent (stale _returnvalue))
    (Variables|Default|SetIsOpen false)
    (else
      (bind _returnvalue (UserInterface|CreateWidget "/Game/Narrative/TextWidgets/StartingHallLetter.StartingHallLetter_C" (Game|GetPlayerController 0)))
      (Appearance|SetBrushfromTexture (Variables|/Game/Narrative/TextWidgets/StartingHallLetter.StartingHallLetter_C|GetImage_16 _returnvalue) (Variables|Default|GetNoteImage) false)
      (Variables|Default|SetWidget _returnvalue)
      (UserInterface|Viewport|AddtoViewport _returnvalue 0)
      (Variables|Default|SetIsOpen true))))