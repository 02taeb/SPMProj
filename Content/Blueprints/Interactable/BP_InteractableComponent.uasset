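; Interactable component that, on Interact, is meant to turn its owning actor around the yaw axis.
; ReturnRInterpOwner runs RInterpTo from the owner's rotation toward that yaw plus RotateDegrees, keeping roll and pitch, with RotateTime as interp speed.
; Interact applies the result in a single SetActorRotation call, with no tick or timeline.
; DeltaTime is left unset on the interpolation, so no gradual turn is driven here.
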(event EventInteract
  (params (Instigator :type Actor%20Object%20Reference))
  (Transformation|SetActorRotation (Components|GetOwner) (CallFunction|ReturnRInterpOwner)))

(fn ReturnRInterpOwner
  (bind _returnvalue (Components|GetOwner))
  (bind _returnvalue_2 (Transformation|GetActorRotation _returnvalue))
  (return (Math|Interpolation|RInterpTo (Math|Rotator|MakeRotator (.roll _returnvalue_2) (.pitch _returnvalue_2) (.yaw _returnvalue_2)) (Math|Rotator|MakeRotator (.roll _returnvalue_2) (.pitch _returnvalue_2) (+ (.yaw _returnvalue_2) (Variables|Default|GetRotateDegrees))) 0.0 (Variables|Default|GetRotateTime))))