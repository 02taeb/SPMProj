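; BP_Corpse is an interactable corpse that shows the player a prompt to eat it; the eating itself is not handled in this graph.
; Entering the InteractPrompt component creates a WBP_InteractPrompt widget if Create is set, with key text chosen by the player's UsingGamepad flag.
; Any end overlap removes every top-level prompt widget of that class, without checking which actor left.
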(event OnComponentBeginOverlap(InteractPrompt)
  (params (OverlappedComponent :type Primitive%20Component%20Object%20Reference) (OtherActor :type Actor%20Object%20Reference) (OtherComp :type Primitive%20Component%20Object%20Reference) (OtherBodyIndex :type Integer) (bFromSweep :type Boolean) (SweepResult :type Hit%20Result%20Structure%20%28by%20ref%29))
  ;[1 1 1] Hugo
  (if (Variables|Default|GetCreate)
    (bind _asplayer_character (Utilities|Casting|CastToPlayerCharacter OtherActor))
    (bind _asplayer_controller (Utilities|Casting|CastToPlayerController (Pawn|GetController _asplayer_character)))
    (bind _returnvalue (UserInterface|CreateWidget "/Game/Blueprints/UI/WBP_InteractPrompt.WBP_InteractPrompt_C" _asplayer_controller))
    (bind _asbp_player_character (Utilities|Casting|CastToBP_PlayerCharacter (Pawn|GetControlledPawn _asplayer_controller)))
    (if (Variables|/Game/Blueprints/PlayerCharacter/BP_PlayerCharacter.BP_PlayerCharacter_C|GetUsingGamepad _asbp_player_character)
      (Variables|/Script/UMG.TextBlock|SetText (Variables|/Game/Blueprints/UI/WBP_InteractPrompt.WBP_InteractPrompt_C|GetText _returnvalue) "Press 'X' to eat corpse")
      (else
        (Variables|/Script/UMG.TextBlock|SetText (Variables|/Game/Blueprints/UI/WBP_InteractPrompt.WBP_InteractPrompt_C|GetText _returnvalue) "Press 'E' to eat corpse")))
    (UserInterface|Viewport|AddtoViewport _returnvalue 0)))

(event OnComponentEndOverlap(InteractPrompt)
  (params (OverlappedComponent :type Primitive%20Component%20Object%20Reference) (OtherActor :type Actor%20Object%20Reference) (OtherComp :type Primitive%20Component%20Object%20Reference) (OtherBodyIndex :type Integer))
  ;[1 1 1] Hugo
  (bind _foundwidgets (Widget|GetAllWidgetsOfClass "/Game/Blueprints/UI/WBP_InteractPrompt.WBP_InteractPrompt_C" true))
  (for _array_element _foundwidgets
    (Widget|RemovefromParent _array_element)))

(fn ConstructionScript)