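; BP_Movable is an interactable object whose mesh the player can push while standing in one of its two axis collision volumes.
; Overlap events on XAxisCollision and YAxisCollision enable physics simulation on the mesh when a PlayerCharacter enters and disable it on exit.
; PushingX and PushingY flags act as a mutual lock, so each volume ignores overlaps while the other axis is being pushed.
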(event OnComponentBeginOverlap(YAxisCollision)
  (params (OverlappedComponent :type Primitive%20Component%20Object%20Reference) (OtherActor :type Actor%20Object%20Reference) (OtherComp :type Primitive%20Component%20Object%20Reference) (OtherBodyIndex :type Integer) (bFromSweep :type Boolean) (SweepResult :type Hit%20Result%20Structure%20%28by%20ref%29))
  ;[1 1 1] Hugo, Collision for Y-Axis
  (if (not (Variables|Default|GetPushingX))
    (Utilities|Casting|CastToPlayerCharacter OtherActor)
    (Physics|SetSimulatePhysics (Variables|Default|GetMesh) true)
    (Variables|Default|SetPushingY true)))

(event OnComponentBeginOverlap(XAxisCollision)
  (params (OverlappedComponent :type Primitive%20Component%20Object%20Reference) (OtherActor :type Actor%20Object%20Reference) (OtherComp :type Primitive%20Component%20Object%20Reference) (OtherBodyIndex :type Integer) (bFromSweep :type Boolean) (SweepResult :type Hit%20Result%20Structure%20%28by%20ref%29))
  ;[1 1 1] Hugo, Collision for X-Axis
  (if (not (Variables|Default|GetPushingY))
    (Utilities|Casting|CastToPlayerCharacter OtherActor)
    (Physics|SetSimulatePhysics (Variables|Default|GetMesh) true)
    (Variables|Default|SetPushingX true)))

(event OnComponentEndOverlap(YAxisCollision)
  (params (OverlappedComponent :type Primitive%20Component%20Object%20Reference) (OtherActor :type Actor%20Object%20Reference) (OtherComp :type Primitive%20Component%20Object%20Reference) (OtherBodyIndex :type Integer))
  ;[1 1 1] Hugo, Collision for Y-Axis
  (if (not (Variables|Default|GetPushingX))
    (Utilities|Casting|CastToPlayerCharacter OtherActor)
    (Physics|SetSimulatePhysics (Variables|Default|GetMesh) false)
    (Variables|Default|SetPushingY false)))

(event OnComponentEndOverlap(XAxisCollision)
  (params (OverlappedComponent :type Primitive%20Component%20Object%20Reference) (OtherActor :type Actor%20Object%20Reference) (OtherComp :type Primitive%20Component%20Object%20Reference) (OtherBodyIndex :type Integer))
  ;[1 1 1] Hugo, Collision for X-Axis
  (if (not (Variables|Default|GetPushingY))
    (Utilities|Casting|CastToPlayerCharacter OtherActor)
    (Physics|SetSimulatePhysics (Variables|Default|GetMesh) false)
    (Variables|Default|SetPushingX false)))

(fn ConstructionScript)