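; BP_Item is a pickup that adds itself to the player's inventory when a PlayerCharacter overlaps it.
; The overlap event casts the other actor, passes the item actor itself to the Inventory's AddItem, then hides Sphere and disables collision on both sphere components.
; Overlap events on Sphere1 are also switched off, and the actor is not destroyed, so the inventory receives a live actor reference.
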(event EventBeginPlay)

(event Collision|EventActorBeginOverlap
  (params (OtherActor :type Actor%20Object%20Reference))
  (bind _asplayer_character (Utilities|Casting|CastToPlayerCharacter OtherActor))
  (Class|InventoryComponent|AddItem (Variables|/Script/SPMProj.PlayerCharacter|GetInventory _asplayer_character) self)
  (Rendering|SetVisibility (Variables|Default|GetSphere) false false)
  (Collision|SetCollisionEnabled (Variables|Default|GetSphere) "NoCollision")
  (Collision|SetCollisionEnabled (Variables|Default|GetSphere1) "NoCollision")
  (Variables|/Script/Engine.PrimitiveComponent|SetbGenerateOverlapEvents (Variables|Default|GetSphere1) false))

(event EventTick
  (params (DeltaSeconds :type Float%20%28single-precision%29)))

(fn ConstructionScript)