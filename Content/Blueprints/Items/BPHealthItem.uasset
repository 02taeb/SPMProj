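; BPHealthItem is a health item pickup that goes into the player's inventory when touched.
; On actor overlap with a PlayerCharacter, it passes itself to that character's Inventory through AddItem.
; It then hides the Cube mesh and turns off collision and Box overlap events, so the actor stays alive as the inventory entry instead of being destroyed.
; No healing logic is in these graphs.
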(event EventBeginPlay)

(event Collision|EventActorBeginOverlap
  (params (OtherActor :type Actor%20Object%20Reference))
  (bind _asplayer_character (Utilities|Casting|CastToPlayerCharacter OtherActor))
  (Class|InventoryComponent|AddItem (Variables|/Script/SPMProj.PlayerCharacter|GetInventory _asplayer_character) self)
  (Rendering|SetVisibility (Variables|Default|GetCube self) false false)
  (Collision|SetCollisionEnabled (Variables|Default|GetBox) "NoCollision")
  (Collision|SetCollisionEnabled (Variables|Default|GetCube) "NoCollision")
  (Variables|/Script/Engine.PrimitiveComponent|SetbGenerateOverlapEvents (Variables|Default|GetBox) false))

(event EventTick
  (params (DeltaSeconds :type Float%20%28single-precision%29)))

(fn ConstructionScript)