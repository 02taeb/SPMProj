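; Player character Blueprint handling HUD creation, death and respawn, healing effects, footsteps and the pause menu.
; BeginPlay adds the UI and loads the save when resuming, while a one-shot on Tick finds and auto-equips the HP, ATK and stamina parasites.
; Death resets UI indicators, ragdolls the mesh and fades out; respawn restores the capsule and mesh and fades in.
; Older inventory and parasite-toggle logic remains disconnected.
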(event Input|EnhancedActionEvents|EnhancedInputActionIA_PauseMeny
  (params (ActionValue :type Boolean) (ElapsedSeconds :type Float%20%28double-precision%29) (TriggeredSeconds :type Float%20%28double-precision%29) (InputAction :type Input%20Action%20Object%20Reference :default "/Game/Input/IA_PauseMeny.IA_PauseMeny"))
  (bind _returnvalue (Game|GetPlayerController 0))
  (bind _returnvalue_2 (Game|GetPlayerController 0))
  (:Started
    (if (Variables|Default|GetCanOpenMenu)
      (if (not (Variables|Default|GetisMenuOpen))
        (Variables|Default|SetisMenuOpen true)
        (bind _returnvalue_3 (UserInterface|CreateWidget "/Game/Blueprints/UI/WBP_PauseMeny.WBP_PauseMeny_C" _returnvalue_2))
        (bind _output_get (Variables|Default|SetPauseMenuWidget _returnvalue_3))
        (UserInterface|Viewport|AddtoViewport _output_get 0)
        (Input|SetInputModeGameandUI _returnvalue_2 (Variables|Default|GetPauseMenuWidget) "DoNotLock" true false)
        (Variables|/Script/Engine.PlayerController|SetbShowMouseCursor (Game|GetPlayerController 0) true)
        (Game|SetGamePaused true)
        (if (Variables|Default|GetUsingGamepad)
          (Widget|SetFocus (Variables|/Game/Blueprints/UI/WBP_PauseMeny.WBP_PauseMeny_C|GetResume (Variables|Default|GetPauseMenuWidget))))
        (else
          (Variables|Default|SetisMenuOpen false)
          (Widget|RemovefromParent (Variables|Default|GetPauseMenuWidget))
          (Game|SetGamePaused false)
          (Input|SetInputModeGameOnly _returnvalue false)
          (Variables|/Script/Engine.PlayerController|SetbShowMouseCursor _returnvalue false))))))

(event Input|EnhancedActionEvents|EnhancedInputActionIA_MoveForward
  (params (ActionValue :type Float%20%28double-precision%29) (ElapsedSeconds :type Float%20%28double-precision%29) (TriggeredSeconds :type Float%20%28double-precision%29) (InputAction :type Input%20Action%20Object%20Reference :default "/Game/Input/IA_MoveForward.IA_MoveForward"))
  ;[1 1 1] Spela footsteps
  (:Started
    (if (not (or (Variables|Default|GetPlayingFootstepsRight) (Variables|Default|GetPlayingFootstepsForward)))
      (Class|PlayerCharacter|PlayFootsteps true)
      (Variables|Default|SetPlayingFootstepsForward true)))
  (:Canceled
    (if (Variables|Default|GetPlayingFootstepsForward)
      (Class|PlayerCharacter|PlayFootsteps false)
      (Variables|Default|SetPlayingFootstepsForward false)))
  (:Completed
    (if (Variables|Default|GetPlayingFootstepsForward)
      (Class|PlayerCharacter|PlayFootsteps false)
      (Variables|Default|SetPlayingFootstepsForward false))))

(event Input|EnhancedActionEvents|EnhancedInputActionIA_MoveRight
  (params (ActionValue :type Float%20%28double-precision%29) (ElapsedSeconds :type Float%20%28double-precision%29) (TriggeredSeconds :type Float%20%28double-precision%29) (InputAction :type Input%20Action%20Object%20Reference :default "/Game/Input/IA_MoveRight.IA_MoveRight"))
  ;[1 1 1] Spela footsteps
  (:Started
    (if (not (or (Variables|Default|GetPlayingFootstepsForward) (Variables|Default|GetPlayingFootstepsRight)))
      (Class|PlayerCharacter|PlayFootsteps true)
      (Variables|Default|SetPlayingFootstepsRight true)))
  (:Canceled
    (if (Variables|Default|GetPlayingFootstepsRight)
      (Class|PlayerCharacter|PlayFootsteps false)
      (Variables|Default|SetPlayingFootstepsRight false)))
  (:Completed
    (if (Variables|Default|GetPlayingFootstepsRight)
      (Class|PlayerCharacter|PlayFootsteps false)
      (Variables|Default|SetPlayingFootstepsRight false))))

(event EventBeginPlay
  ;[1 1 1] Hugo
  (bind _returnvalue (UserInterface|CreateWidget "/Game/Blueprints/UI/WPB_UI.WPB_UI_C" (Game|GetPlayerController 0)))
  (UserInterface|Viewport|AddtoViewport _returnvalue 0)
  (bind _asbp_game_instance (Utilities|Casting|CastToBP_GameInstance (Game|GetGameInstance)))
  (if (Variables|/Game/Blueprints/GameInstance/BP_GameInstance.BP_GameInstance_C|GetResumed _asbp_game_instance)
    (bind _asbp_player_character (Utilities|Casting|CastToBP_PlayerCharacter (Game|Player|GetPlayerPawn 0)))
    (Class|PlayerCharacter|LoadGame _asbp_player_character)))

(event EventOnHeal
  (bind _healingdecal (Variables|Default|GetHealingDecal))
  (Utilities|IsValid (Variables|Default|GetHealingSystem)
    (:Is%20Valid
      (Components|DestroyComponent (Variables|Default|GetHealingSystem)))
    (:Is%20Not%20Valid
      _))
  (Utilities|IsValid _healingdecal
    (:Is%20Valid
      (Actor|DestroyActor _healingdecal))
    (:Is%20Not%20Valid
      _))
  (bind _returnvalue (Niagara|SpawnSystematLocation "/Game/VFX_Thöz/Öz/HEALING_CIRCLE/NS_Healing_Plus.NS_Healing_Plus" (Transformation|GetActorLocation) "0, 0, 0" "1.000000,1.000000,1.000000" false))
  (bind _output_get (Variables|Default|SetHealingSystem _returnvalue))
  (Utilities|FlowControl|Delay 3.0)
  (Components|DestroyComponent _output_get))

(event EventTick
  (params (DeltaSeconds :type Float%20%28single-precision%29))
  (Utilities|FlowControl|DoOnce false
    (:Completed
      (CallFunction|SetHPParRef)
      (CallFunction|SetATKParRef)
      (CallFunction|SetSTMParRef))))

(event EventOnDeathBPEvent
  (Utilities|FlowControl|Sequence
    (:then_0
      (bind _foundwidgets (Widget|GetAllWidgetsOfClass "/Game/Blueprints/UI/WPB_UI.WPB_UI_C" true))
      (Default|UpdateATK (Utilities|Array|Get(acopy) _foundwidgets) false)
      (Default|UpdateHP (Utilities|Array|Get(acopy) _foundwidgets) false)
      (Default|UpdateSTM (Utilities|Array|Get(acopy) _foundwidgets) false))
    (:then_1
      (CallFunction|Ragdoll)
      (CameraFades|StartCameraFade :self (Game|GetPlayerCameraManager 0) :ToAlpha 1.0 :Duration 0.5 :bHoldWhenFinished true))))

(event EventOnRespawnBPEvent
  (bind _returnvalue (Game|GetPlayerCameraManager 0))
  (CallFunction|ResetRagdoll)
  (Audio|PlaySound2D 0 1.0 1.0 0.0 0 0)
  (CameraFades|StopCameraFade _returnvalue)
  (CameraFades|StartCameraFade :self _returnvalue :FromAlpha 1.0 :Duration 0.5))

(event Input|KeyboardEvents|0
  (params (Key :type Key%20Structure :default "None"))
  (:Pressed
    (Class|PlayerCharacter|KillSelf)))

(event Input|KeyboardEvents|3
  (params (Key :type Key%20Structure :default "None"))
  ;[1 1 1] Deprecated, pars should always be equipped
)

(event Input|KeyboardEvents|1
  (params (Key :type Key%20Structure :default "None"))
  ;[1 1 1] Deprecated, pars should always be equipped
)

(event Input|KeyboardEvents|2
  (params (Key :type Key%20Structure :default "None"))
  ;[1 1 1] Deprecated, pars should always be equipped
)

(event Input|KeyboardEvents|AnyKey
  (params (Key :type Key%20Structure :default "None"))
  ;[1 1 1] kanske används för gamepad specifik behaviour
  (:Pressed
    (if (Class|KismetInputLibrary|KeyIsGamepadKey Key)
      (Variables|Default|SetUsingGamepad true)
      (else
        (Variables|Default|SetUsingGamepad false)))))

(fn ConstructionScript)

(fn SetHPParRef
  (bind _outactors (Actor|GetAllActorsOfClass "/Game/Blueprints/Items/Parasites/BP_HPParasite.BP_HPParasite_C"))
  (bind _output_get (Variables|Default|SetHPPar (Utilities|Array|Get(acopy) _outactors)))
  (bind _asequipable_parasite (Utilities|Casting|CastToEquipableParasite _output_get))
  (Variables|/Script/SPMProj.EquipableParasite|SetPlayerActorPtr _asequipable_parasite self)
  (Class|EquipableParasite|OnPickup _asequipable_parasite)
  (Class|EquipableParasite|OnEquip _asequipable_parasite))

(fn SetATKParRef
  (bind _outactors (Actor|GetAllActorsOfClass "/Game/Blueprints/Items/Parasites/BP_AtkParasite.BP_AtkParasite_C"))
  (bind _output_get (Variables|Default|SetATKPar (Utilities|Array|Get(acopy) _outactors)))
  (bind _asequipable_parasite (Utilities|Casting|CastToEquipableParasite _output_get))
  (Variables|/Script/SPMProj.EquipableParasite|SetPlayerActorPtr _asequipable_parasite self)
  (Class|EquipableParasite|OnPickup _asequipable_parasite)
  (Class|EquipableParasite|OnEquip _asequipable_parasite))

(fn SetSTMParRef
  (bind _outactors (Actor|GetAllActorsOfClass "/Game/Blueprints/Items/Parasites/BP_StmParasite.BP_StmParasite_C"))
  (bind _output_get (Variables|Default|SetSTMPar (Utilities|Array|Get(acopy) _outactors)))
  (bind _asequipable_parasite (Utilities|Casting|CastToEquipableParasite _output_get))
  (Variables|/Script/SPMProj.EquipableParasite|SetPlayerActorPtr _asequipable_parasite self)
  (Class|EquipableParasite|OnPickup _asequipable_parasite)
  (Class|EquipableParasite|OnEquip _asequipable_parasite))

(fn Ragdoll
  (bind _mesh (Variables|Character|GetMesh))
  (Pawn|Components|CharacterMovement|SetMovementMode (Variables|Character|GetCharacterMovement) "MOVE_None" 0)
  (Collision|SetCollisionEnabled (Variables|Default|GetCapsuleComponent) "NoCollision")
  (Collision|SetCollisionObjectType _mesh "ECC_PhysicsBody")
  (Collision|SetCollisionEnabled _mesh "QueryAndPhysics")
  (Class|SkeletalMeshComponent|SetAllBodiesSimulatePhysics _mesh true))

(fn ResetRagdoll
  (bind _capsulecomponent (Variables|Default|GetCapsuleComponent))
  (bind _mesh (Variables|Character|GetMesh))
  (Pawn|Components|CharacterMovement|SetMovementMode (Variables|Character|GetCharacterMovement) "MOVE_Walking" 0)
  (Collision|SetCollisionEnabled _capsulecomponent "QueryAndPhysics")
  (Collision|SetCollisionObjectType _mesh "ECC_WorldDynamic")
  (Collision|SetCollisionEnabled _mesh "QueryOnly")
  (Class|SkeletalMeshComponent|SetAllBodiesSimulatePhysics _mesh false)
  (Transformation|SetWorldLocation _capsulecomponent (Transformation|GetWorldLocation _mesh) false false)
  (Transformation|AttachComponentToComponent _mesh _capsulecomponent "None" "SnapToTarget" "KeepRelative" "KeepRelative" true)
  (Transformation|SetRelativeLocation _mesh "0.000000,0.000000,-95.000000" false false)
  (Transformation|SetRelativeRotation _mesh "0.000000,-90.000000,0.000000" false false))