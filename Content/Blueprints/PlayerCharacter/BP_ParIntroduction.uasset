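; BP_ParIntroduction is a trigger actor that shows an introduction widget while the player is inside its box.
; On overlap by the PlayerCharacter, it creates WBP_ParIntroduction, plays the note-open sound, and switches to Game and UI input with a visible cursor.
; When any overlap ends, without checking the actor, it removes the widget and restores game-only input with a hidden cursor for player zero.
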(event OnComponentBeginOverlap(Box)
  (params (OverlappedComponent :type Primitive%20Component%20Object%20Reference) (OtherActor :type Actor%20Object%20Reference) (OtherComp :type Primitive%20Component%20Object%20Reference) (OtherBodyIndex :type Integer) (bFromSweep :type Boolean) (SweepResult :type Hit%20Result%20Structure%20%28by%20ref%29))
  (bind _asplayer_character (Utilities|Casting|CastToPlayerCharacter OtherActor))
  (bind _asplayer_controller (Utilities|Casting|CastToPlayerController (Pawn|GetController _asplayer_character)))
  (bind _returnvalue (UserInterface|CreateWidget "/Game/Blueprints/UI/WBP_ParIntroduction.WBP_ParIntroduction_C" _asplayer_controller))
  (bind _output_get (Variables|Default|SetWidget _returnvalue))
  (UserInterface|Viewport|AddtoViewport _output_get 0)
  (Input|SetInputModeGameandUI _asplayer_controller _output_get "DoNotLock" true false)
  (Variables|/Script/Engine.PlayerController|SetbShowMouseCursor _asplayer_controller true)
  (Audio|PlaySound2D "/Game/Audio/Interact/Note_Open.Note_Open" 1.0 1.0 0.0 0 0))

(event OnComponentEndOverlap(Box)
  (params (OverlappedComponent :type Primitive%20Component%20Object%20Reference) (OtherActor :type Actor%20Object%20Reference) (OtherComp :type Primitive%20Component%20Object%20Reference) (OtherBodyIndex :type Integer))
  (bind _returnvalue (Game|GetPlayerController 0))
  (Widget|RemovefromParent (Variables|Default|GetWidget))
  (Input|SetInputModeGameOnly _returnvalue false)
  (Variables|/Script/Engine.PlayerController|SetbShowMouseCursor _returnvalue false))

(fn ConstructionScript)