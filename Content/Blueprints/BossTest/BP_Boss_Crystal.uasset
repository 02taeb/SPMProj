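; BP_Boss_Crystal is a crystal actor, apparently for a boss test, that changes its glow when struck by a melee weapon.
; The construction script creates and stores a dynamic material instance from the static mesh's first material slot.
; On overlap with a MeleeWeapon, it sets that material's Emissive Strength to the Emissive variable, which the graph never modifies.
; Debug prints report the value or a failed cast.
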(event EventBeginPlay)

(event Collision|EventActorBeginOverlap
  (params (OtherActor :type Actor%20Object%20Reference))
  (bind _emissive (Variables|Default|GetEmissive))
  (Utilities|Casting|CastToMeleeWeapon OtherActor
    (:then
      (Rendering|Material|SetScalarParameterValue (Variables|Default|GetVar) "Emissive Strength" _emissive :!class /Script/Engine.MaterialInstanceDynamic)
      (Development|PrintString (Utilities|String|ToString(Float) _emissive)))
    (:CastFailed
      (Development|PrintString "Cast Failed!"))))

(event EventTick
  (params (DeltaSeconds :type Float%20%28single-precision%29)))

(fn ConstructionScript
  (bind _returnvalue (Rendering|Material|CreateDynamicMaterialInstance (Variables|Debug|GetStaticMeshComponent) 0 0 "None" :!class /Script/Engine.PrimitiveComponent))
  (Variables|Default|SetVar _returnvalue))