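; BP_EnemyTeleport is a teleporting enemy that ragdolls on death and can then be interacted with.
; BeginPlay sets the ShouldTeleport blackboard key, and Tick switches the Niagara teleport effect on or off from a flag.
; Hits raise a damage parameter on the mesh materials.
; Death enables mesh physics, ignores pawn and camera collision, and shows an interact prompt to overlapping players, with box overlaps adding or removing it afterwards.
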(event OnComponentBeginOverlap(Box)
  (params (OverlappedComponent :type Primitive%20Component%20Object%20Reference) (OtherActor :type Actor%20Object%20Reference) (OtherComp :type Primitive%20Component%20Object%20Reference) (OtherBodyIndex :type Integer) (bFromSweep :type Boolean) (SweepResult :type Hit%20Result%20Structure%20%28by%20ref%29))
  ;[1 1 1] Interact prompt
  (if (Variables|Default|GetIsDead)
    (bind _asbp_player_character (Utilities|Casting|CastToBP_PlayerCharacter OtherActor))
    (bind _asplayer_controller (Utilities|Casting|CastToPlayerController (Pawn|GetController _asbp_player_character)))
    (bind _returnvalue (UserInterface|CreateWidget "/Game/Blueprints/UI/WBP_InteractPrompt.WBP_InteractPrompt_C" _asplayer_controller))
    (bind _output_get (Variables|Default|SetWidget _returnvalue))
    (UserInterface|Viewport|AddtoViewport _output_get 0)
    (Variables|Default|SetWidgetCreated true)))

(event OnComponentEndOverlap(Box)
  (params (OverlappedComponent :type Primitive%20Component%20Object%20Reference) (OtherActor :type Actor%20Object%20Reference) (OtherComp :type Primitive%20Component%20Object%20Reference) (OtherBodyIndex :type Integer))
  ;[1 1 1] Interact prompt
  (bind _foundwidgets (Widget|GetAllWidgetsOfClass "/Game/Blueprints/UI/WBP_InteractPrompt.WBP_InteractPrompt_C" true))
  (for _array_element _foundwidgets
    (Widget|RemovefromParent _array_element))
  (Variables|Default|SetWidgetCreated false))

(event OnComponentActivated(Niagara_TeleportEffect)
  (params (Component :type Actor%20Component%20Object%20Reference) (bReset :type Boolean)))

(event EventOnDeathBPEvent
  (bind _capsulecomponent (Variables|Default|GetCapsuleComponent))
  ;[1 1 1] Ragdoll
  (Physics|SetSimulatePhysics (Variables|Character|GetMesh) true)
  (Pawn|Components|CharacterMovement|DisableMovement (Variables|Character|GetCharacterMovement))
  (Variables|Default|SetIsDead true)
  (Collision|SetCollisionResponsetoChannel _capsulecomponent "ECC_Pawn" "ECR_Ignore")
  (Collision|SetCollisionResponsetoChannel _capsulecomponent "ECC_Camera" "ECR_Ignore")
  (bind _array_element (Utilities|Array|ForEachLoopwithBreak (Collision|GetOverlappingActors (Variables|Default|GetBox) 0 :!class /Script/Engine.PrimitiveComponent) :!label _label)
    (:LoopBody
      (bind _asbp_player_character (Utilities|Casting|CastToBP_PlayerCharacter _array_element))
      (bind _asplayer_controller (Utilities|Casting|CastToPlayerController (Pawn|GetController _asbp_player_character)))
      (bind _returnvalue (UserInterface|CreateWidget "/Game/Blueprints/UI/WBP_InteractPrompt.WBP_InteractPrompt_C" _asplayer_controller))
      (bind _output_get (Variables|Default|SetWidget _returnvalue))
      (UserInterface|Viewport|AddtoViewport _output_get 0)
      (Variables|Default|SetWidgetCreated true)
      (goto _label Break))))

(event EventOnHitBPEvent
  (bind _output_get (Variables|Default|SetDamageValue (+ (Variables|Default|GetDamageValue) (Variables|Default|GetOnHitMatInc))))
  (Rendering|Material|SetScalarParameterValueonMaterials (Variables|Character|GetMesh) "Damge_taken" _output_get))

(event EventBeginPlay
  (AI|Components|Blackboard|SetValueasBool (AI|GetBlackboard 0) (Utilities|Name|MakeLiteralName "ShouldTeleport") true))

(event EventTick
  (params (DeltaSeconds :type Float%20%28single-precision%29))
  (bind _niagara_teleporteffect (Variables|Default|GetNiagara_TeleportEffect))
  (if (Variables|Default|GetShouldTeleportEffectPlay)
    (Components|Activation|Activate _niagara_teleporteffect false)
    (else
      (Components|Activation|Deactivate _niagara_teleporteffect))))

(fn ConstructionScript)