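; Patrol enemy Blueprint that shows accumulated damage on its mesh and becomes an interactable ragdoll on death.
; Each hit event raises a damage value that drives a material scalar parameter.
; Death enables mesh physics, disables movement and makes the capsule ignore Pawn and Camera channels.
; The box shows an interact prompt to overlapping players once dead, including any already inside at death, and removes it when they leave.
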(event OnComponentBeginOverlap(Box)
  (params (OverlappedComponent :type Primitive%20Component%20Object%20Reference) (OtherActor :type Actor%20Object%20Reference) (OtherComp :type Primitive%20Component%20Object%20Reference) (OtherBodyIndex :type Integer) (bFromSweep :type Boolean) (SweepResult :type Hit%20Result%20Structure%20%28by%20ref%29))
  ;[1 1 1] Interact prompt
  (if (Variables|Default|GetIsDead)
    (bind _asbp_player_character (Utilities|Casting|CastToBP_PlayerCharacter OtherActor))
    (bind _asplayer_controller (Utilities|Casting|CastToPlayerController (Pawn|GetController _asbp_player_character)))
    (bind _returnvalue (UserInterface|CreateWidget "/Game/Blueprints/UI/WBP_InteractPrompt.WBP_InteractPrompt_C" _asplayer_controller))
    (bind _output_get (Variables|Default|SetWidget _returnvalue))
    (UserInterface|Viewport|AddtoViewport _output_get 0)
    (Variables|Default|SetWidgetCreated true)))

(event OnComponentEndOverlap(Box)
  (params (OverlappedComponent :type Primitive%20Component%20Object%20Reference) (OtherActor :type Actor%20Object%20Reference) (OtherComp :type Primitive%20Component%20Object%20Reference) (OtherBodyIndex :type Integer))
  ;[1 1 1] Interact prompt
  (if (Variables|Default|GetWidgetCreated)
    (Utilities|Casting|CastToBP_PlayerCharacter OtherActor)
    (Widget|RemovefromParent (Variables|Default|GetWidget))
    (Variables|Default|SetWidgetCreated false)))

(event EventOnDeathBPEvent
  (bind _capsulecomponent (Variables|Default|GetCapsuleComponent))
  ;[1 1 1] Ragdoll
  (Physics|SetSimulatePhysics (Variables|Character|GetMesh) true)
  (Pawn|Components|CharacterMovement|DisableMovement (Variables|Character|GetCharacterMovement))
  (Variables|Default|SetIsDead true)
  (Collision|SetCollisionResponsetoChannel _capsulecomponent "ECC_Pawn" "ECR_Ignore")
  (Collision|SetCollisionResponsetoChannel _capsulecomponent "ECC_Camera" "ECR_Ignore")
  (bind _array_element (Utilities|Array|ForEachLoopwithBreak (Collision|GetOverlappingActors (Variables|Default|GetBox) 0 :!class /Script/Engine.PrimitiveComponent) :!label _label)
    (:LoopBody
      (bind _asbp_player_character (Utilities|Casting|CastToBP_PlayerCharacter _array_element))
      (bind _asplayer_controller (Utilities|Casting|CastToPlayerController (Pawn|GetController _asbp_player_character)))
      (bind _returnvalue (UserInterface|CreateWidget "/Game/Blueprints/UI/WBP_InteractPrompt.WBP_InteractPrompt_C" _asplayer_controller))
      (bind _output_get (Variables|Default|SetWidget _returnvalue))
      (UserInterface|Viewport|AddtoViewport _output_get 0)
      (Variables|Default|SetWidgetCreated true)
      (goto _label Break))))

(event EventOnHitBPEvent
  (bind _output_get (Variables|Default|SetDamageValue (+ (Variables|Default|GetDamageValue) (Variables|Default|GetOnHitMatInc))))
  (Rendering|Material|SetScalarParameterValueonMaterials (Variables|Character|GetMesh) "Damge_taken" _output_get))

(fn ConstructionScript)