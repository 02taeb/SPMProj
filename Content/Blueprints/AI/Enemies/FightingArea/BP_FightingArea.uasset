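; BP_FightingArea marks a fighting area's door with a blood decal that responds to the number of enemies left alive.
; Each EnemiesLeft event destroys the current decal, then spawns a replacement if three, two or one enemies remain.
; All three branches currently use the same material and size.
; The Values helper supplies the door's static mesh, bounds origin and world rotation for attaching the decal.
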(event EventEnemiesLeft
  (params (EnemiesAlive :type Integer))
  (bind (_returnvalue _returnvalue2 _returnvalue3) (CallFunction|Values))
  (bind (_returnvalue_2 _returnvalue2_2 _returnvalue3_2) (CallFunction|Values))
  (bind (_returnvalue_3 _returnvalue2_3 _returnvalue3_3) (CallFunction|Values))
  (Components|DestroyComponent (Variables|Default|GetDecal))
  (if (== EnemiesAlive 3)
    (bind _returnvalue_4 (Class|GameplayStatics|SpawnDecalAttached "/Game/VFX_Thöz/Öz/Blood_Splatter_Pool/Decal_blood_M_Inst1.Decal_blood_M_Inst1" "100.000000,100.000000,100.000000" _returnvalue_2 "None" _returnvalue2_2 _returnvalue3_2 "KeepWorldPosition" 0.0))
    (Variables|Default|SetDecal _returnvalue_4)
    (elif (== EnemiesAlive 2)
      (bind _returnvalue_5 (Class|GameplayStatics|SpawnDecalAttached "/Game/VFX_Thöz/Öz/Blood_Splatter_Pool/Decal_blood_M_Inst1.Decal_blood_M_Inst1" "100.000000,100.000000,100.000000" _returnvalue_3 "None" _returnvalue2_3 _returnvalue3_3 "KeepWorldPosition" 0.0))
      (Variables|Default|SetDecal _returnvalue_5)
      (elif (== EnemiesAlive 1)
        (bind _returnvalue_6 (Class|GameplayStatics|SpawnDecalAttached "/Game/VFX_Thöz/Öz/Blood_Splatter_Pool/Decal_blood_M_Inst1.Decal_blood_M_Inst1" "100.000000,100.000000,100.000000" _returnvalue "None" _returnvalue2 _returnvalue3 "KeepWorldPosition" 0.0))
        (Variables|Default|SetDecal _returnvalue_6)))))

(fn ConstructionScript)

(fn Values
  (bind _door (Variables|Default|GetDoor))
  (bind _returnvalue (Actor|GetComponentbyClass _door "/Script/Engine.StaticMeshComponent"))
  (return _returnvalue (.Origin (Collision|GetComponentBounds _returnvalue)) (Transformation|GetWorldRotation _returnvalue)))