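; Melee weapon actor with a pickup zone and hit effects, likely a sword.
; Entering the zone shows a gamepad-aware interact prompt; leaving it sets the player's HasSword if unset and, once, shows a combat intro and clears the prompt.
; Each hit spawns an FS_MasterField at the impact point, then triggers the target's blood-effect component (a separate variant for Enemy actors) with a hit sound.
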(event OnComponentBeginOverlap(PickupZone)
  (params (OverlappedComponent :type Primitive%20Component%20Object%20Reference) (OtherActor :type Actor%20Object%20Reference) (OtherComp :type Primitive%20Component%20Object%20Reference) (OtherBodyIndex :type Integer) (bFromSweep :type Boolean) (SweepResult :type Hit%20Result%20Structure%20%28by%20ref%29))
  (bind _asbp_player_character (Utilities|Casting|CastToBP_PlayerCharacter OtherActor))
  (bind _returnvalue (UserInterface|CreateWidget "/Game/Blueprints/UI/WBP_InteractPrompt.WBP_InteractPrompt_C" (Game|GetPlayerController 0)))
  (if (Variables|/Game/Blueprints/PlayerCharacter/BP_PlayerCharacter.BP_PlayerCharacter_C|GetUsingGamepad _asbp_player_character)
    (Variables|/Script/UMG.TextBlock|SetText (Variables|/Game/Blueprints/UI/WBP_InteractPrompt.WBP_InteractPrompt_C|GetText _returnvalue) "Press 'X' to pick up weapon")
    (else
      (Variables|/Script/UMG.TextBlock|SetText (Variables|/Game/Blueprints/UI/WBP_InteractPrompt.WBP_InteractPrompt_C|GetText _returnvalue) "Press 'E' to pick up weapon")))
  (UserInterface|Viewport|AddtoViewport _returnvalue 0))

(event OnComponentEndOverlap(PickupZone)
  (params (OverlappedComponent :type Primitive%20Component%20Object%20Reference) (OtherActor :type Actor%20Object%20Reference) (OtherComp :type Primitive%20Component%20Object%20Reference) (OtherBodyIndex :type Integer))
  (bind _asbp_player_character (Utilities|Casting|CastToBP_PlayerCharacter OtherActor))
  (if (not (Variables|/Game/Blueprints/PlayerCharacter/BP_PlayerCharacter.BP_PlayerCharacter_C|GetHasSword _asbp_player_character))
    (Variables|/Game/Blueprints/PlayerCharacter/BP_PlayerCharacter.BP_PlayerCharacter_C|SetHasSword _asbp_player_character true)
    (Utilities|FlowControl|DoOnce false
      (:Completed
        (bind _returnvalue (UserInterface|CreateWidget "/Game/Narrative/MechanicIntroductions/CombatIntro/CombatIntroFixed.CombatIntroFixed_C"))
        (UserInterface|Viewport|AddtoViewport _returnvalue 0)
        (Widget|RemovefromParent (stale OnComponentBeginOverlap(PickupZone) _returnvalue))))))

(event EventOnHit
  (params (HitActor :type Actor%20Object%20Reference) (HitLocation :type Vector :default "0, 0, 0") (HitResult :type Hit%20Result%20Structure))
  (bind _returnvalue (Actor|GetComponentbyClass HitActor "/Game/VFX_Thöz/Öz/Blood_Splatter_Pool/Fiendens_Blod/AC_Blood_Effect_2.AC_Blood_Effect_2_C"))
  (bind _returnvalue_2 (Actor|GetComponentbyClass HitActor "/Game/VFX_Thöz/Öz/Blood_Splatter_Pool/Spelarens_blod/AC_Blood_Effect.AC_Blood_Effect_C"))
  (Game|SpawnActorfromClass "/Engine/EditorResources/FieldNodes/FS_MasterField.FS_MasterField_C" (Math|Transform|MakeTransform HitLocation) "Undefined" 0 0)
  (Utilities|Casting|CastToEnemy HitActor
    (:then
      (if (Utilities|IsValid HitActor)
        (if (Utilities|IsValid _returnvalue)
          (Default|ActivateBloodEffect _returnvalue HitLocation (.Normal (Collision|BreakHitResult HitResult)))
          (Audio|PlaySoundatLocation "/Game/Sound/SFX/SwordHit.SwordHit" (Transformation|GetActorLocation) "0, 0, 0" 1.0 1.0 0.0 0 0 0 0))))
    (:CastFailed
      (if (Utilities|IsValid HitActor)
        (if (Utilities|IsValid _returnvalue_2)
          (Default|ActivateBloodEffect _returnvalue_2 HitLocation (.Normal (Collision|BreakHitResult HitResult)))
          (Audio|PlaySoundatLocation "/Game/Sound/SFX/SwordHit.SwordHit" (Transformation|GetActorLocation) "0, 0, 0" 1.0 1.0 0.0 0 0 0 0))))))

(fn ConstructionScript)